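; BP_Sink is a sink actor that takes in dishes, apparently as part of a collection mission.
; When an actor implementing both IDishes and ICollectable overlaps its Box, the sink hides it and updates CustomGameMode, lowering CollectablesLeft and raising DishCount.
; Disconnected leftover nodes hold a MaxDishes check and a GameManager dish counter, neither of which runs.
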(event OnComponentBeginOverlap(Box)
  (params (OverlappedComponent :type Primitive%20Component%20Object%20Reference) (OtherActor :type Actor%20Object%20Reference) (OtherComp :type Primitive%20Component%20Object%20Reference) (OtherBodyIndex :type Integer) (bFromSweep :type Boolean) (SweepResult :type Hit%20Result%20Structure%20%28by%20ref%29))
  (if (and (Utilities|DoesObjectImplementInterface OtherActor "/Game/BPs/Interfaces/IDishes.IDishes_C") (Utilities|DoesObjectImplementInterface OtherActor "/Game/BPs/Interfaces/ICollectable.ICollectable_C"))
    (Rendering|SetActorHiddenInGame OtherActor true)
    (bind _ascustom_game_mode (Utilities|Casting|CastToCustomGameMode (Game|GetGameMode)))
    (Variables|Default|SetcustomGameModeRef _ascustom_game_mode)
    (bind _result (Math|Integer|DecrementInt (Variables|/Game/Testing/CustomGameMode.CustomGameMode_C|GetCollectablesLeft _ascustom_game_mode))
      (:%20%20
        (Variables|/Game/Testing/CustomGameMode.CustomGameMode_C|SetCollectablesLeft _ascustom_game_mode _result)
        (bind _result_2 (Math|Integer|IncrementInt (Variables|/Game/Testing/CustomGameMode.CustomGameMode_C|GetdishCount _ascustom_game_mode))
          (:%20%20
            (Variables|/Game/Testing/CustomGameMode.CustomGameMode_C|SetdishCount _ascustom_game_mode _result_2)))))))

(event EventBeginPlay)

(event Collision|EventActorBeginOverlap
  (params (OtherActor :type Actor%20Object%20Reference)))

(event EventTick
  (params (DeltaSeconds :type Float%20%28single-precision%29)))

(fn ConstructionScript)